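; BP_Sun is a sun actor with a point light whose source radius is set through an event.
; SetRadiusEvent multiplies the incoming Radius by a Scale variable and applies the result to the PointLight's source radius.
; BeginPlay, overlap and Tick are disabled stubs, and the construction script only calls its parent.
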(event `self.SetRadiusEvent`
  (params (Radius :type "Float (double-precision) (by ref)"))
  (`PointLightComponent.SetSourceRadius` (`self.PointLight`) (* Radius (`self.Scale`))))

(fn `UserConstructionScript`
  (`parent.UserConstructionScript`))