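; BP_Asteroid is an asteroid actor that selects its static mesh from its Name value when play begins.
; BeginPlay looks up Name in the AsteroidsNormalized map of a newly made AsteroidMap and applies the matching mesh to Body, falling back to the normalized Bennu mesh.
; It prints the name and lookup result on screen, while the construction script only calls its parent.
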(event `self.ReceiveBeginPlay`
  (bind _name (`self.Name`))
  (bind (_value _returnvalue) (`BlueprintMapLibrary.Map_Find` (`.asteroids_normalized_19_7313ECFE234C834682FBEF880F07A60C` (break `/Game/AsteroidMeshes/asteroid_map` (make `/Game/AsteroidMeshes/asteroid_map` _))) _name))
  (`parent.ReceiveBeginPlay`)
  (`KismetSystemLibrary.PrintString` _name true true (struct :`G` 0.66 :`B` 1.0 :`A` 1.0) 5.0)
  (if _returnvalue
    (`KismetSystemLibrary.PrintText` "Found!" true true (struct :`G` 0.66 :`B` 1.0 :`A` 1.0) 5.0)
    (`StaticMeshComponent.SetStaticMesh` (`self.Body`) _value)
    (else
      (`KismetSystemLibrary.PrintText` "Not Found" true true (struct :`G` 0.66 :`B` 1.0 :`A` 1.0) 5.0)
      (`StaticMeshComponent.SetStaticMesh` (`self.Body`) "/Game/AsteroidMeshes/bennu_normalized.bennu_normalized"))))

(fn `UserConstructionScript`
  (`parent.UserConstructionScript`))