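; BP_Spacecraft is a spacecraft actor that carries a configurable onboard camera built on a SceneCaptureComponent2D.
; Custom events set the camera's relative position, orientation and field of view, and resize its target render texture to a given resolution.
; GenerateCameraImage captures the scene into that render target on demand, and DrawCoordinates draws debug axes at a capture component's world transform.
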(event `self.SetCameraPosition`
  (params (Position :type "Vector Structure (by ref)"))
  (`SceneComponent.K2_SetRelativeLocation` (`self.SceneCaptureComponent2D`) Position false false))

(event `self.UpdateCameraOrientation`
  (params (Orientation :type "Rotator Structure (by ref)"))
  (`SceneComponent.K2_SetRelativeRotation` (`self.SceneCaptureComponent2D`) Orientation false false))

(event `self.SetFOV`
  (params (X :type "Float (double-precision)") (Y :type "Float (double-precision)"))
  (set `SceneCaptureComponent2D.FOVAngle` X (`self.SceneCaptureComponent2D`)))

(event `self.SetResolution`
  (params (ResolutionWidth :type Integer) (ResolutionHeight :type Integer))
  (`KismetRenderingLibrary.ResizeRenderTarget2D` (`SceneCaptureComponent2D.TextureTarget` (`self.SceneCaptureComponent2D`)) ResolutionWidth ResolutionHeight))

(fn `Draw Coordinates`
  (params (CaptureComponent :type "SceneComponent Object Reference"))
  (`KismetSystemLibrary.DrawDebugCoordinateSystem` (`SceneComponent.K2_GetComponentLocation` CaptureComponent) (`SceneComponent.K2_GetComponentRotation` CaptureComponent)))

(fn `Generate Camera Image`
  (`SceneCaptureComponent2D.CaptureScene` (`self.SceneCaptureComponent2D`)))

(fn `UserConstructionScript`)